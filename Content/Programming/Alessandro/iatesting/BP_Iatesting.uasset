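; Test enemy AI pawn with Tank montages that roams around BP_Tree, attacking it or the player.
; Distance-check macros drive an AIMoveTo loop, with a looping timer switching to chasing when the player is near.
; Attacks use a rotation timeline and random left/right montage sections; hand-socket sphere traces apply damage by Player or Tree tag.
; Damage triggers a hit reaction and renewed chase, or death with randomly scattered BP_Exp drops.
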(event Custom|LoopCheck
  (Utilities|ChasePlayer?
    (:True
      (CallFunction|ChasePlayer)
      (Utilities|Time|ClearandInvalidateTimerbyHandle (stale Custom|GoToTree _returnvalue)))))

(event Custom|GoToTree
  (AI|AIMoveTo self (.RandomLocation (AI|Navigation|GetRandomReachablePointinRadius (Variables|Default|GetTreelocation) 7.5e+03 0 0)) 0 5.0 false :!label _label
    (:then
      (bind _returnvalue (Utilities|Time|SetTimerbyEvent (delegate Custom|LoopCheck) 0.1 true)))
    (:OnSuccess
      (Utilities|ChasePlayer? :!label _label_2
        (:True
          (CallFunction|ChasePlayer))
        (:False
          (Utilities|HastoAttackTree?
            (:True
              (CallFunction|Attack))
            (:False
              (goto _label))))))
    (:OnFail
      (goto _label_2))))

(event Custom|ChasePlayer
  (AI|AIMoveTo self "0, 0, 0" (Game|GetPlayerCharacter 0) 9e+01 false :!label _label
    (:OnSuccess
      (Utilities|HastoAttackPlayer?
        (:True
          (CallFunction|Attack))
        (:False
          (Utilities|ChasePlayer? :!label _label_2
            (:True
              (goto _label))
            (:False
              (CallFunction|GotoTree))))))
    (:OnFail
      (goto _label_2))))

(event Custom|SphereTraceStart
  (bind _handsocket (Variables|Default|GethandSocket))
  (bind _mesh (Variables|Character|GetMesh))
  (bind _returnvalue (Transformation|GetSocketLocation _mesh _handsocket))
  (bind (_outhits _returnvalue_2) (Collision|MultiSphereTraceByChannel _returnvalue _returnvalue 5e+01 "TraceTypeQuery1" false 0 "Persistent"))
  (if _returnvalue_2
    (for _array_element _outhits
      (if (Actor|ActorHasTag (.hitactor _array_element) "Player")
        (Utilities|FlowControl|DoOnce false :!label _label
          (:Completed
            (Game|Damage|ApplyDamage (.hitactor _array_element) -1e+02 0 0)
            (Utilities|FlowControl|Delay 0.5)
            (goto _label Reset)))
        (elif (Actor|ActorHasTag (.hitactor _array_element) "Tree")
          (Utilities|FlowControl|DoOnce false :!label _label_2
            (:Completed
              (Game|Damage|ApplyDamage 0 -1e+01 0 0)
              (Utilities|FlowControl|Delay 0.5)
              (goto _label_2 Reset))))))))

(event Custom|Attack
  (bind _returnvalue (Transformation|GetActorLocation))
  (bind _targetloc (Variables|Default|Gettargetloc))
  (bind _returnvalue_2 (- _targetloc _returnvalue))
  (bind _returnvalue_3 (Math|Vector|Normalize _returnvalue_2))
  (bind _returnvalue_4 (Math|Conversions|RotationFromXVector _returnvalue_3))
  (Variables|Default|SetcurrentRot (Transformation|GetActorRotation))
  (bind _alpha (Timeline|LerpRotation PlayFromStart)
    (:Update
      (Transformation|SetActorRotation (Math|Rotator|Lerp(Rotator) (Variables|Default|GetcurrentRot) (Math|Rotator|MakeRotator (.roll _returnvalue_4) (.pitch (Variables|Default|GetcurrentRot)) (+ (.yaw _returnvalue_4) 0.0)) _alpha true))
      (if (Math|Random|RandomBool)
        (Variables|Default|SetattkSlotName "AttackL")
        (Variables|Default|SethandSocket "hand_lSocket")
        (else
          (Variables|Default|SetattkSlotName "AttackR")
          (Variables|Default|SethandSocket "hand_rSocket")))
      (Animation|Montage|PlayMontage (Variables|Character|GetMesh) "/Game/Programming/Alessandro/Test/Tank/Animation/Attack/TankAttack.TankAttack" 1.0 0.0 (Variables|Default|GetattkSlotName)
        (:OnCompleted
          (Utilities|HastoAttackPlayer?
            (:True
              (CallFunction|Attack :!label _label))
            (:False
              (Utilities|ChasePlayer?
                (:True
                  (CallFunction|ChasePlayer))
                (:False
                  (Utilities|HastoAttackTree?
                    (:True
                      (goto _label))
                    (:False
                      (CallFunction|GotoTree))))))))))))

(event Game|Damage|EventAnyDamage
  (params (Damage :type Float%20%28single-precision%29) (DamageType :type Damage%20Type%20Object%20Reference) (InstigatedBy :type Controller%20Object%20Reference) (DamageCauser :type Actor%20Object%20Reference))
  (bind _returnvalue (Transformation|GetActorLocation))
  (bind _returnvalue_2 (Math|Random|RandomIntegerinRange 0 5))
  (bind _mesh (Variables|Character|GetMesh))
  (Variables|Default|SettakeDamage true)
  (bind _output_get (Variables|Default|SetcurrentHP (- (Variables|Default|GetcurrentHP) Damage)))
  (if (<= _output_get 0.0)
    (Utilities|FlowControl|DoOnce false
      (:Completed
        (Animation|Montage|PlayMontage _mesh "/Game/Programming/Alessandro/Test/Tank/Animation/Dead/TankDeadMontage.TankDeadMontage"
          (:then
            (Utilities|FlowControl|Delay 1.0)
            (for _index (range 0 _returnvalue_2)
              (bind _returnvalue_3 (Game|SpawnActorfromClass "/Game/Programming/MainBP/BP_Exp.BP_Exp_C" (Math|Transform|MakeTransform (Math|Vector|MakeVector (+ (.x _returnvalue) (Math|Random|RandomFloatinRange -1e+02 1e+02)) (+ (.y _returnvalue) (Math|Random|RandomFloatinRange -2e+02 2e+02)) (+ (.z _returnvalue) (Math|Random|RandomFloatinRange -5e+01 75.0))) "0, 0, 0" "1.000000,1.000000,1.000000") "Undefined" 0 0))
              (Variables|/Game/Programming/MainBP/BP_Exp.BP_Exp_C|SetXp%20to%20Add _returnvalue_3 (/ (Variables|Default|GetXpToDrop) _returnvalue_2)))))))
    (else
      (Animation|Montage|PlayMontage _mesh "/Game/Programming/Alessandro/Test/Tank/Animation/React/tankReactMontage.tankReactMontage"
        (:OnCompleted
          (Variables|Default|SettakeDamage false)
          (CallFunction|ChasePlayer))))))

(event EventBeginPlay
  (bind _returnvalue (Actor|GetActorOfClass "/Game/Programming/MainBP/BP_Tree.BP_Tree_C"))
  (Variables|Default|SetTreelocation (Transformation|GetActorLocation _returnvalue))
  (CallFunction|GotoTree))

(fn ConstructionScript)