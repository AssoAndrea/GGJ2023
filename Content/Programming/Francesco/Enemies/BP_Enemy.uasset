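; Melee enemy character that attacks the mage and BP_Target, with hit and death reactions.
; Attack sphere-traces for victims and plays a random left or right montage, temporarily enabling that side's damage collider.
; Damage reduces HP and writes the blackboard; death awards weight as XP and spawner points, then notifies the game mode.
; A looping timer scales HP and damage up but zeroes the other EnemyValues fields, including weight and attack speed.
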(event OnComponentBeginOverlap(rSphereCollider)
  (params (OverlappedComponent :type Primitive%20Component%20Object%20Reference) (OtherActor :type Actor%20Object%20Reference) (OtherComp :type Primitive%20Component%20Object%20Reference) (OtherBodyIndex :type Integer) (bFromSweep :type Boolean) (SweepResult :type Hit%20Result%20Structure%20%28by%20ref%29))
  (Utilities|Casting|CastToBP_Mage OtherActor
    (:then
      _)
    (:CastFailed
      (Utilities|Casting|CastToBP_Target OtherActor)))
  (bind _result (Math|Float|NegateFloat (.damage (Variables|Default|GetenemyValues)))
    (:%20%20
      (Game|Damage|ApplyDamage OtherActor _result 0 0))))

(event OnComponentBeginOverlap(lSphereCollider)
  (params (OverlappedComponent :type Primitive%20Component%20Object%20Reference) (OtherActor :type Actor%20Object%20Reference) (OtherComp :type Primitive%20Component%20Object%20Reference) (OtherBodyIndex :type Integer) (bFromSweep :type Boolean) (SweepResult :type Hit%20Result%20Structure%20%28by%20ref%29))
  (Utilities|Casting|CastToBP_Mage OtherActor
    (:then
      _)
    (:CastFailed
      (Utilities|Casting|CastToBP_Target OtherActor)))
  (bind _result (Math|Float|NegateFloat (.damage (Variables|Default|GetenemyValues)))
    (:%20%20
      (Game|Damage|ApplyDamage OtherActor _result 0 0))))

(event Custom|CustomEvent
  (Variables|Default|SetenemyValues (Utilities|Struct|MakeST_Enemies_Stats (* (.hp (Variables|Default|GetenemyValues)) 1.1) (* (.damage (Variables|Default|GetenemyValues)) 1.1) 0.0 0.0 0 0.0)))

(event Custom|PlayMontage
  (Utilities|PlayAttackMontage))

(event EventBeginPlay
  (bind _asggj_game_mode (Utilities|Casting|CastToGGJ_GameMode (Game|GetGameMode)))
  (Variables|Default|SetgameMode _asggj_game_mode)
  (Collision|SetCollisionEnabled (Variables|Default|GetlSphereCollider) "NoCollision")
  (Utilities|Time|SetTimerbyEvent (delegate Custom|CustomEvent) 2e+01 true))

(event Game|Damage|EventAnyDamage
  (params (Damage :type Float%20%28single-precision%29) (DamageType :type Damage%20Type%20Object%20Reference) (InstigatedBy :type Controller%20Object%20Reference) (DamageCauser :type Actor%20Object%20Reference))
  (bind _gamemode (Variables|Default|GetgameMode))
  (bind _mesh (Variables|Character|GetMesh))
  (if (<= (.hp (Variables|Default|GetenemyValues)) 0.0)
    (Collision|SetCollisionEnabled (Variables|Collision|GetCapsuleComponent) "NoCollision")
    (Collision|SetCollisionEnabled (Variables|Character|GetMesh) "NoCollision")
    (Utilities|FlowControl|DoOnce false
      (:Completed
        (Animation|Montage|PlayMontage _mesh (Variables|Default|GetdeathMontage)
          (:OnCompleted
            (Default|AddXp _gamemode (.weight (Variables|Default|GetenemyValues)))
            (bind _returnvalue (Actor|GetActorOfClass "/Game/Programming/Francesco/Enemies/Spawner/SpawnerTimeManager.SpawnerTimeManager_C"))
            (bind _output_get (Variables|Default|SetspawnerTimeManager _returnvalue))
            (Variables|/Game/Programming/Francesco/Enemies/Spawner/SpawnerTimeManager.SpawnerTimeManager_C|Setpoints _output_get (+ (.weight (Variables|Default|GetenemyValues)) (Variables|/Game/Programming/Francesco/Enemies/Spawner/SpawnerTimeManager.SpawnerTimeManager_C|Getpoints _output_get)))
            (Default|CallOnKilledEnemy _gamemode)))))
    (else
      (AI|Components|Blackboard|SetValueasBool (AI|GetBlackboard (AI|GetAIController self)) (Utilities|Name|MakeLiteralName "haveBeenAttacked") false)
      (Variables|Default|SetenemyValues (Utilities|Struct|MakeST_Enemies_Stats (- (.hp (Variables|Default|GetenemyValues)) Damage) (.damage (Variables|Default|GetenemyValues)) (.attackdelay (Variables|Default|GetenemyValues)) (.attackspeed (Variables|Default|GetenemyValues)) (.velocity (Variables|Default|GetenemyValues)) (.weight (Variables|Default|GetenemyValues))))
      (Animation|Montage|PlayMontage _mesh (Variables|Default|GethitMontage)))))

(fn ConstructionScript)

(fn Attack
  (bind _returnvalue (Transformation|GetActorLocation))
  (if (Math|Random|RandomBool)
    (Variables|Default|SetattackSectionName "AttackL")
    (else
      (Variables|Default|SetattackSectionName "AttackR")))
  (bind (_outhits _returnvalue_2) (Collision|MultiSphereTraceForObjects _returnvalue _returnvalue 1.2e+02 (Utilities|Array|MakeArray "ObjectTypeQuery3" "ObjectTypeQuery7") false 0 "None"))
  (if _returnvalue_2
    (bind _index (Utilities|FlowControl|ForLoopwithBreak 0 (Utilities|Array|Length _outhits) :!label _label)
      (:LoopBody
        (Utilities|Casting|CastToBP_Mage (.hitactor (Utilities|Array|Get(acopy) _outhits _index))
          (:then
            _)
          (:CastFailed
            (bind _asbp_target (Utilities|Casting|CastToBP_Target (.hitactor (Utilities|Array|Get(acopy) _outhits _index))))
            (Transformation|SetActorRotation (Math|Rotator|MakeRotator 0.0 0.0 (.yaw (Math|Rotator|FindLookatRotation (Transformation|GetActorLocation self) (Transformation|GetActorLocation _asbp_target)))))))
        (CallFunction|PlayMontage)
        (goto _label Break)))))