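; BP_Tree is an actor with HP that ends in a death screen when depleted.
; Heal/DamageTree adds a flat or MaxHP-percentage value to HP, unclamped; its HP print is unreachable.
; AnyDamage passes damage unnegated, so positive values raise HP; at zero or below, it shows BP_DEAD once with UI-only input and cursor.
; SetGamePaused receives false, and the OnTreeDefeated dispatcher call is never reached.
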(event Custom|Heal/Damage%20Tree
  (params (Value :type Float%20%28double-precision%29) (IsPercentage :type Boolean))
  (bind _output_get (Variables|Default|SetHP (Math|Float|SelectFloat (+ (Variables|Default|GetHP) (* (/ Value 1e+02) (Variables|Default|GetMaxHP))) (+ (Variables|Default|GetHP) Value) IsPercentage)))
  (if (<= _output_get 0.0)
    _
    (else
      _))
  (Development|PrintString (Utilities|String|ToString(Float) (Variables|Default|GetHP))))

(event EventBeginPlay)

(event Collision|EventActorBeginOverlap
  (params (OtherActor :type Actor%20Object%20Reference)))

(event EventTick
  (params (DeltaSeconds :type Float%20%28single-precision%29)))

(event Game|Damage|EventAnyDamage
  (params (Damage :type Float%20%28single-precision%29) (DamageType :type Damage%20Type%20Object%20Reference) (InstigatedBy :type Controller%20Object%20Reference) (DamageCauser :type Actor%20Object%20Reference))
  (bind _returnvalue (Game|GetPlayerController 0))
  (CallFunction|Heal/DamageTree Damage false)
  (if (<= (Variables|Default|GetHP) 0.0)
    (Utilities|FlowControl|DoOnce false
      (:Completed
        (bind _returnvalue_2 (UserInterface|CreateWidget "/Game/Programming/Antonino/Help/HUD/BP_DEAD.BP_DEAD_C"))
        (UserInterface|Viewport|AddtoViewport _returnvalue_2 0)
        (Input|SetInputModeUIOnly _returnvalue _returnvalue_2 "LockAlways" false)
        (Variables|/Script/Engine.PlayerController|SetbShowMouseCursor _returnvalue true)
        (Game|SetGamePaused false)))))

(fn ConstructionScript)